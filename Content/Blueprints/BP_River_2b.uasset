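; BP_River_2b is a river hazard that kills the player chicken and clears away actors that reach its despawn point.
; MurderBox overlap spawns a BP_DeadChicken and a lowered splash effect at the player, hands controller possession to the corpse, then destroys the player.
; A Running flag latches after the first kill to prevent repeats, resetting only for non-player overlaps.
; DespawnPoint destroys any actor that overlaps it.
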(event `self.DespawnPoint.OnComponentBeginOverlap`
  (params (OverlappedComponent :type "PrimitiveComponent Object Reference") (OtherActor :type "Actor Object Reference") (OtherComp :type "PrimitiveComponent Object Reference") (OtherBodyIndex :type Integer) (bFromSweep :type Boolean) (SweepResult :type "HitResult Structure (by ref)"))
  (`self.K2_DestroyActor` OtherActor))

(event `self.MurderBox.OnComponentBeginOverlap`
  (params (OverlappedComponent :type "PrimitiveComponent Object Reference") (OtherActor :type "Actor Object Reference") (OtherComp :type "PrimitiveComponent Object Reference") (OtherBodyIndex :type Integer) (bFromSweep :type Boolean) (SweepResult :type "HitResult Structure (by ref)"))
  (if (== (`self.Running`) 1)
    (set `self.Running` 0)
    (bind _asbp_player_chicken (cast `/Game/ThirdPersonBP/Blueprints/BP_PlayerChicken` OtherActor)
      (:`then`
        (bind _returnvalue (`self.GetTransform` _asbp_player_chicken))
        (bind _returnvalue_2 (`|SpawnActorFromClass` "/Game/ThirdPersonBP/Blueprints/BP_DeadChicken.BP_DeadChicken_C" _returnvalue "Undefined" "OverrideRootScale" null null))
        (`GameplayStatics.SpawnEmitterAtLocation` "/Game/ThirdPersonBP/Particles/Splash.Splash" (`KismetMathLibrary.MakeVector` (.x (.location _returnvalue)) (.y (.location _returnvalue)) (- (.z (.location _returnvalue)) 50.0)) (.rotation _returnvalue) (.scale _returnvalue))
        (`Controller.Possess` (`Pawn.GetController` _asbp_player_chicken) _returnvalue_2)
        (`self.K2_DestroyActor` _asbp_player_chicken))
      (:`CastFailed`
        (set `self.Running` 1)))))

(fn `UserConstructionScript`)