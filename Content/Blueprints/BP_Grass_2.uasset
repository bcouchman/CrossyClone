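; BP_Grass_2 is a grass Blueprint that spawns randomized trees through its SpawnTree function at a supplied transform.
; A coin flip places either one BP_BigTree at that transform or two BP_SmallTrees offset to either side on X with random stepped Y jitter.
; The second small tree subtracts the base Y from its jitter, so its Y is mirrored around the world origin.
; The event graph and construction script are empty.
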(event `self.ReceiveBeginPlay`)

(fn `SpawnTree`
  (params (NewParam :type "Transform Structure"))
  (bind _rotation (.rotation NewParam))
  (bind _scale (.scale NewParam))
  (bind _returnvalue (* (`KismetMathLibrary.RandomIntegerInRange` -10 10) 10.0))
  (if (`KismetMathLibrary.RandomBool`)
    (`|SpawnActorFromClass` "/Game/ThirdPersonBP/Blueprints/BP_BigTree.BP_BigTree_C" NewParam "Undefined" "OverrideRootScale" null null)
    (else
      (`|SpawnActorFromClass` "/Game/ThirdPersonBP/Blueprints/BP_SmallTree.BP_SmallTree_C" (`KismetMathLibrary.MakeTransform` (`KismetMathLibrary.MakeVector` (- (.x (.location NewParam)) 90.0) (+ _returnvalue (.y (.location NewParam))) (.z (.location NewParam))) _rotation _scale) "Undefined" "OverrideRootScale" null null)
      (`|SpawnActorFromClass` "/Game/ThirdPersonBP/Blueprints/BP_SmallTree.BP_SmallTree_C" (`KismetMathLibrary.MakeTransform` (`KismetMathLibrary.MakeVector` (+ (.x (.location NewParam)) 90.0) (- _returnvalue (.y (.location NewParam))) (.z (.location NewParam))) _rotation _scale) "Undefined" "OverrideRootScale" null null))))

(fn `UserConstructionScript`)